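; Actor component in the Dynamic Combat System that resolves animation montages for requested actions from data tables.
; The owner supplies a table per action through I_MontageManagerComponent, with a warning on BeginPlay if unimplemented.
; GetAction records the last request, scans rows by Action field and falls back to a default table.
; Last-index and random-index helpers instead look up rows by enum name in the owner's table only, without that fallback.
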(event EventBeginPlay
  (if (not (Utilities|DoesObjectImplementInterface (Components|GetOwner) "/Game/DynamicCombatSystem/Blueprints/Interfaces/I_MontageManagerComponent.I_MontageManagerComponent_C"))
    (Development|PrintString (Utilities|String|Append "Warning! " (Utilities|GetClassDisplayName (Utilities|GetClass (Components|GetOwner))) " does not implement interface I_MontageManager") true true "(R=1.000000,G=0.974717,B=0.000000,A=1.000000)" 5.0)))

(fn GetMontageforAction
  (params (Action :type E_MontageAction%20Enum :default "NewEnumerator35") (Index :type Integer))
  (bind (_isfound _action) (CallFunction|GetAction Action))
  (if _isfound
    (if (Utilities|Array|IsValidIndex (Utilities|Struct|BreakF_MontageAction _action) Index)
      (return (Utilities|Array|Get(acopy) (Utilities|Struct|BreakF_MontageAction _action) Index))
      (else
        (return 0)))
    (else
      (return 0))))

(fn GetMontageActionLastIndex
  (params (Action :type E_MontageAction%20Enum :default "NewEnumerator35"))
  (bind _returnvalue (Utilities|GetMontage123123 Action)
    (:RowFound
      (return (Utilities|Array|LastIndex (Utilities|Struct|BreakF_MontageAction _returnvalue))))
    (:RowNotFound
      (return -1))))

(fn GetRandomMontageIndex
  (params (MontageAction :type E_MontageAction%20Enum :default "NewEnumerator35"))
  (return (Math|Random|RandomIntegerinRange 0 (CallFunction|GetMontageActionLastIndex MontageAction))))

(fn GetLastRequestedAction
  (return (Variables|Default|GetLastRequestedAction)))

(fn GetAction
  (params (ActionType :type E_MontageAction%20Enum :default "NewEnumerator35"))
  (bind _output_get (Variables|Default|SetLastRequestedAction ActionType))
  (bind _montages (Class|IMontageManagerComponent|GetMontages(Message) (Components|GetOwner) _output_get))
  (bind (_isfound _out_row) (CallFunction|GetActionfromTable _montages ActionType))
  (if _isfound
    (return _isfound _out_row)
    (else
      (bind (_isfound_2 _out_row_2) (CallFunction|GetActionfromTable (Variables|Default|GetDefaultMontageActionsDataTable) ActionType))
      (return _isfound_2 _out_row_2))))

(fn GetActionfromTable
  (params (TableToSearch :type Data%20Table%20Object%20Reference) (ActionType :type E_MontageAction%20Enum :default "NewEnumerator35"))
  (Utilities|IsValid TableToSearch
    (:Is%20Valid
      (bind _outrownames (DataTable|GetDataTableRowNames TableToSearch))
      (for _array_element _outrownames
        (bind _returnvalue (Utilities|GetDataTableRow TableToSearch _array_element)
          (:then
            (if (Utilities|Enum|Equal(Enum) (Utilities|Struct|BreakF_MontageAction _returnvalue) ActionType)
              (return true _returnvalue)))
          (:RowNotFound
            (return false "")))))
    (:Is%20Not%20Valid
      _))
  (return false ""))